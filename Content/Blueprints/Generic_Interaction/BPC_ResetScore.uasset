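; BPC_ResetScore is an interactable actor Blueprint that resets the target spawner's scores.
; On Interacted, it finds all BP_TargetSpawner actors, takes the first, and calls ResetHighScore and ResetToZero on it.
; Its BeginPlay, overlap and Tick events are disabled, and the construction script only calls its parent, so the interaction is its only active logic.
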(event EventBeginPlay
  (|CallParentFunction) ; This node is disabled and will not be called.\nDrag off pins to build functionality.
)

(event Collision|EventActorBeginOverlap
  (params (OtherActor :type Actor%20Object%20Reference)))

(event EventTick
  (params (DeltaSeconds :type Float%20%28single-precision%29))
  (|CallParentFunction DeltaSeconds) ; This node is disabled and will not be called.\nDrag off pins to build functionality.
)

(event EventInteracted
  (bind _outactors (Actor|GetAllActorsOfClass "/Game/_Mechanics/_Target/BP_TargetSpawner.BP_TargetSpawner_C"))
  (bind _asbp_target_spawner (Utilities|Casting|CastToBP_TargetSpawner (Utilities|Array|Get(acopy) _outactors)))
  (Default|ResetHighScore _asbp_target_spawner)
  (Default|ResettoZero _asbp_target_spawner))

(fn ConstructionScript
  (|CallParentFunction))