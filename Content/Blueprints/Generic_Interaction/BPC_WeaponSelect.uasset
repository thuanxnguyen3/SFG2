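; BPC_WeaponSelect is an interactable weapon selector that equips the player with its configured weapon class.
; The construction script applies the Weapon class to its BPWeapon child actor component, so the actor displays that weapon.
; On Interacted, it sets the same class on the Weapon child actor component of BP_FirstPersonCharacter_Target, then adds a WB_FlashEffect widget to the viewport.
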(event EventBeginPlay
  (|CallParentFunction) ; This node is disabled and will not be called.\nDrag off pins to build functionality.
)

(event Collision|EventActorBeginOverlap
  (params (OtherActor :type Actor%20Object%20Reference)))

(event EventTick
  (params (DeltaSeconds :type Float%20%28single-precision%29))
  (|CallParentFunction DeltaSeconds) ; This node is disabled and will not be called.\nDrag off pins to build functionality.
)

(event EventInteracted
  (Utilities|FlowControl|Sequence
    (:then_0
      (bind _asbp_first_person_character_target (Utilities|Casting|CastToBP_FirstPersonCharacter_Target (Game|GetPlayerCharacter 0)))
      (ChildActorComponent|SetChildActorClass (Variables|/Game/Blueprints/FirstPersonTemplate/BP_FirstPersonCharacter_Target.BP_FirstPersonCharacter_Target_C|GetWeapon _asbp_first_person_character_target) (Variables|Default|GetWeapon)))
    (:then_1
      (bind _returnvalue (UserInterface|CreateWidget "/Game/_Mechanics/_UI/WB_FlashEffect.WB_FlashEffect_C" (Game|GetPlayerController 0)))
      (UserInterface|Viewport|AddtoViewport _returnvalue 0))))

(fn ConstructionScript
  (|CallParentFunction)
  (ChildActorComponent|SetChildActorClass (Variables|Default|GetBP_Weapon) (Variables|Default|GetWeapon)))