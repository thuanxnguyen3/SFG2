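; BP_BossBullet is a bullet actor, named for a boss, that deals fixed damage on impact and then destroys itself.
; A sphere hit damages whatever actor was struck, gated only by a cast confirming the player character is BP_FirstPersonCharacter.
; A sphere overlap destroys the bullet without damage; its exclusion requires the other actor to be both player pawn and bullet, so effectively any overlap destroys it.
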(event OnComponentHit(Sphere)
  (params (HitComponent :type Primitive%20Component%20Object%20Reference) (OtherActor :type Actor%20Object%20Reference) (OtherComp :type Primitive%20Component%20Object%20Reference) (NormalImpulse :type Vector :default "0, 0, 0") (Hit :type Hit%20Result%20Structure%20%28by%20ref%29))
  (Utilities|Casting|CastToBP_FirstPersonCharacter (Game|GetPlayerCharacter 0))
  (Game|Damage|ApplyDamage OtherActor 2e+01 0 0)
  (Actor|DestroyActor))

(event OnComponentBeginOverlap(Sphere)
  (params (OverlappedComponent :type Primitive%20Component%20Object%20Reference) (OtherActor :type Actor%20Object%20Reference) (OtherComp :type Primitive%20Component%20Object%20Reference) (OtherBodyIndex :type Integer) (bFromSweep :type Boolean) (SweepResult :type Hit%20Result%20Structure%20%28by%20ref%29))
  (if (not (and (== OtherActor (Game|Player|GetPlayerPawn 0)) (== OtherActor self)))
    (Actor|DestroyActor)))

(fn ConstructionScript)