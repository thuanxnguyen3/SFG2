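; BP_BossTurret is a boss turret that shoots at the first-person player and can be destroyed by damage.
; When PawnSensing sees a BP_FirstPersonCharacter, the turret snaps to face it, then after a short Delay spawns a BP_BossBullet from its Arrow component's transform.
; AnyDamage reduces clamped Health and destroys the actor when it reaches zero, with an IsDead flag guarding further hits.
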(event OnSeePawn(PawnSensing)
  (params (Pawn :type Pawn%20Object%20Reference))
  (Utilities|Casting|CastToBP_FirstPersonCharacter Pawn)
  (Transformation|SetActorRotation (Math|Rotator|FindLookatRotation (Transformation|GetActorLocation) (Transformation|GetActorLocation Pawn)))
  (Utilities|FlowControl|Delay 0.4)
  (Game|SpawnActorfromClass "/Game/_Mechanics/_Turret/BP_BossBullet.BP_BossBullet_C" (Transformation|GetWorldTransform (Variables|Default|GetArrow)) "Undefined" "MultiplyWithRoot" 0 0))

(event Game|Damage|EventAnyDamage
  (params (Damage :type Float%20%28single-precision%29) (DamageType :type Damage%20Type%20Object%20Reference) (InstigatedBy :type Controller%20Object%20Reference) (DamageCauser :type Actor%20Object%20Reference))
  (if (not (Variables|Default|GetIsDead?))
    (bind _output_get (Variables|Default|SetHealth (Math|Float|Clamp(Float) (- (Variables|Default|GetHealth) Damage) 0.0 (Variables|Default|GetMax%20Health))))
    (if (== _output_get 0.0)
      (Actor|DestroyActor)
      (Variables|Default|SetIsDead? true))))

(fn ConstructionScript
  (|CallParentFunction))