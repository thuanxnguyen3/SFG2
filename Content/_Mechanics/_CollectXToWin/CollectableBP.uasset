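; Collectable pickup actor for a collect-X-to-win mechanic, triggered by overlap with its Box.
; On player overlap it decrements CollectablesLeft in BP_FirstPersonGameMode, shows a widget, plays sound and Niagara effects, and destroys itself.
; Every overlap also checks for zero remaining, then spawns win effects, calls Win on the game mode and switches to UI-only input with a cursor.
; End overlap by the first-person character calls DisableInput.
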(event OnComponentEndOverlap(Box)
  (params (OverlappedComponent :type Primitive%20Component%20Object%20Reference) (OtherActor :type Actor%20Object%20Reference) (OtherComp :type Primitive%20Component%20Object%20Reference) (OtherBodyIndex :type Integer))
  (Utilities|Casting|CastToBP_FirstPersonCharacter OtherActor)
  (Input|DisableInput (Game|GetPlayerController 0)))

(event OnComponentBeginOverlap(Box)
  (params (OverlappedComponent :type Primitive%20Component%20Object%20Reference) (OtherActor :type Actor%20Object%20Reference) (OtherComp :type Primitive%20Component%20Object%20Reference) (OtherBodyIndex :type Integer) (bFromSweep :type Boolean) (SweepResult :type Hit%20Result%20Structure%20%28by%20ref%29))
  (bind _returnvalue (Game|GetPlayerController 0))
  (Utilities|FlowControl|Sequence
    (:then_0
      (if (== OtherActor (Game|Player|GetPlayerPawn 0))
        (bind _asbp_first_person_game_mode (Utilities|Casting|CastToBP_FirstPersonGameMode (Game|GetGameMode)))
        (bind _result (Math|Integer|DecrementInt (Variables|/Game/FirstPerson/Blueprints/BP_FirstPersonGameMode.BP_FirstPersonGameMode_C|GetCollectables%20Left _asbp_first_person_game_mode))
          (:%20%20
            (Variables|/Game/FirstPerson/Blueprints/BP_FirstPersonGameMode.BP_FirstPersonGameMode_C|SetCollectables%20Left _asbp_first_person_game_mode _result)
            (bind _returnvalue_2 (UserInterface|CreateWidget "/Game/_Mechanics/_CollectXToWin/CollectableWidget.CollectableWidget_C"))
            (UserInterface|Viewport|AddtoViewport _returnvalue_2 0)
            (Audio|PlaySound2D "/Game/_Mechanics/_CollectXToWin/CollectableSound.CollectableSound" 1.0 1.0 0.0 0 0)
            (Niagara|SpawnSystematLocation "/Game/_Mechanics/_CollectXToWin/FX_Collectable.FX_Collectable" (Transformation|GetActorLocation))
            (Actor|DestroyActor)))))
    (:then_1
      (if true
        (bind _asbp_first_person_game_mode_2 (Utilities|Casting|CastToBP_FirstPersonGameMode (Game|GetGameMode)))
        (if (== (Variables|/Game/FirstPerson/Blueprints/BP_FirstPersonGameMode.BP_FirstPersonGameMode_C|GetCollectables%20Left _asbp_first_person_game_mode_2) 0)
          (Niagara|SpawnSystematLocation "/Game/_Mechanics/_WinScreen/FX_PlayerWin.FX_PlayerWin" (Transformation|GetActorLocation (Game|Player|GetPlayerPawn 0)))
          (Default|Win _asbp_first_person_game_mode_2)
          (Variables|/Script/Engine.PlayerController|SetbShowMouseCursor _returnvalue true)
          (Input|SetInputModeUIOnly _returnvalue 0 "DoNotLock" false))))))

(fn ConstructionScript)