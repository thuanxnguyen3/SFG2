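; BP_WeaponBase is a base weapon Blueprint that manages magazine ammo and provides firing effects.
; Ammo fills to the magazine maximum on BeginPlay, and the ReloadWeapon event refills it after a ReloadTime delay.
; WeaponFireEffects spawns the configured fire emitter and sound at the Arrow component's world transform, which acts as the muzzle point.
; No firing or ammo consumption logic appears in this Blueprint.
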(event Custom|ReloadWeapon
  (Utilities|FlowControl|Delay (Variables|Ammo|GetReloadTime))
  (Variables|Ammo|SetAmmo (Variables|Ammo|GetMaxMagazineAmmo)))

(event EventBeginPlay
  (Variables|Ammo|SetAmmo (Variables|Ammo|GetMaxMagazineAmmo)))

(fn ConstructionScript)

(fn WeaponFireEffects
  (bind _arrow (Variables|Default|GetArrow))
  (bind _returnvalue (Transformation|GetWorldTransform _arrow))
  (Effects|SpawnEmitteratLocation (Variables|WeaponFireEffects|GetWeaponFireEmitter) (.location _returnvalue) (.rotation _returnvalue) (Variables|WeaponFireEffects|GetWeaponFireEmitterScale))
  (Audio|SpawnSoundatLocation (Variables|WeaponFireEffects|GetWeaponFireSound) (.location _returnvalue) "0, 0, 0" 1.0 1.0 0.0 0 0)
  (return))