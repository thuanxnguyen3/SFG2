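; BP_Dummy is a target dummy that briefly flashes when damaged.
; On BeginPlay it creates a dynamic material instance from the DummyPTorus6 component's first material and stores it as FlashMat.
; The Damage event sets that material's emissive color and multiplier to the configured flash values, then resets them to black and zero after a short delay.
; No health or damage amount is tracked here.
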(event EventBeginPlay
  (bind __dummy_ptorus6 (Variables|Default|Get_dummy_pTorus6))
  (bind _returnvalue (Rendering|Material|CreateDynamicMaterialInstance __dummy_ptorus6 0 (Rendering|Material|GetMaterial __dummy_ptorus6 0) "None" :!class /Script/Engine.PrimitiveComponent))
  (Variables|Default|SetFlashMat _returnvalue))

(event EventDamage
  (params (Points :type Integer))
  (bind _flashmat (Variables|Default|GetFlashMat))
  (bind _flashmat_2 (Variables|Default|GetFlashMat))
  (Rendering|Material|SetVectorParameterValue _flashmat_2 "EmissiveColor" (Variables|Default|GetFlashColor) :!class /Script/Engine.MaterialInstanceDynamic)
  (Rendering|Material|SetScalarParameterValue _flashmat_2 "EmissiveMultiplier" (Variables|Default|GetFlashIntensity) :!class /Script/Engine.MaterialInstanceDynamic)
  (Utilities|FlowControl|Delay 0.1)
  (Rendering|Material|SetVectorParameterValue :self _flashmat :ParameterName "EmissiveColor" :!class /Script/Engine.MaterialInstanceDynamic)
  (Rendering|Material|SetScalarParameterValue _flashmat "EmissiveMultiplier" 0.0 :!class /Script/Engine.MaterialInstanceDynamic))

(fn ConstructionScript)