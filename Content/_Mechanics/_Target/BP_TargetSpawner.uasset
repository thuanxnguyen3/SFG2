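; BP_TargetSpawner fills a box volume with BP_Target actors, sized by BoxExtent in the construction script.
; StartSpawning, not BeginPlay, spawns an initial burst and starts a looping timer that calls SpawnTarget.
; SpawnTarget checks the world-wide target count against a cap, then spawns at a random point in the box.
; Each target is rotated toward the player camera with a yaw offset at spawn time.
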(event Custom|SpawnTarget
  (bind _spawn_area (Variables|Default|GetSpawn_Area))
  (bind _outactors (Actor|GetAllActorsOfClass "/Game/_Mechanics/_Target/BP_Target.BP_Target_C"))
  (if (<= (Utilities|Array|Length _outactors) 30)
    (bind _output_get (Variables|Default|SetSpawnLocation (Math|Random|RandomPointinBoundingBox (Transformation|GetWorldLocation _spawn_area) (Components|Box|GetScaledBoxExtent _spawn_area))))
    (Game|SpawnActorfromClass "/Game/_Mechanics/_Target/BP_Target.BP_Target_C" (Math|Transform|MakeTransform _output_get (Math|Rotator|MakeRotator (.roll (Math|Rotator|FindLookatRotation _output_get (Transformation|GetWorldLocation (Variables|/Script/Engine.PlayerCameraManager|GetTransformComponent (Game|GetPlayerCameraManager 0))))) (.pitch (Math|Rotator|FindLookatRotation _output_get (Transformation|GetWorldLocation (Variables|/Script/Engine.PlayerCameraManager|GetTransformComponent (Game|GetPlayerCameraManager 0))))) (- (.yaw (Math|Rotator|FindLookatRotation _output_get (Transformation|GetWorldLocation (Variables|/Script/Engine.PlayerCameraManager|GetTransformComponent (Game|GetPlayerCameraManager 0))))) 9e+01)) "1.000000,1.000000,1.000000") "AdjustIfPossibleButAlwaysSpawn" "MultiplyWithRoot" 0 0)))

(event Custom|StartSpawning
  (Utilities|Time|SetTimerbyEvent (delegate Custom|SpawnTarget) 1.0 true)
  (for _index (range 0 8)
    (CallFunction|SpawnTarget)))

(event EventBeginPlay)

(fn ConstructionScript
  (Components|Box|SetBoxExtent (Variables|Default|GetSpawn_Area) (Variables|Default|GetBoxExtent) true))